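; Game mode that turns audio levels from two MetaSounds, Nyeh and Debussy, into shoot events.
; On BeginPlay it adds an audio component for each track and watches its float output through the MetaSound Output Subsystem.
; When an output reaches that track's threshold, it calls the matching Shoot event.
; A per-track flag and delay act as a cooldown, so sustained loud audio cannot retrigger immediately.
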(event Custom|Nyeh_Out
  (params (OutputName :type Name) (Output :type Meta%20Sound%20Output%20Structure%20%28by%20ref%29))
  (bind (_success _returnvalue) (Class|MetasoundOutputBlueprintAccess|GetFloat Output))
  (if (Math|Boolean|ANDBoolean _success (>= _returnvalue (Variables|Default|GetNyehLevel)) (not (Variables|Default|GetbNyehCalled)))
    (Variables|Default|SetbNyehCalled true)
    (Class|CubeGameModeBase|CallNyehShoot)
    (CallFunction|NyehWaitTime)))

(event Custom|NyehWaitTime
  (Utilities|FlowControl|Delay (Variables|Default|GetWaitTimeNyeh))
  (Variables|Default|SetbNyehCalled false))

(event Custom|Debussy_Out
  (params (OutputName :type Name) (Output :type Meta%20Sound%20Output%20Structure%20%28by%20ref%29))
  (bind (_success _returnvalue) (Class|MetasoundOutputBlueprintAccess|GetFloat Output))
  (if (Math|Boolean|ANDBoolean _success (>= _returnvalue (Variables|Default|GetDebussyLevel)) (not (Variables|Default|GetbDebussyCalled)))
    (Variables|Default|SetbDebussyCalled true)
    (Class|CubeGameModeBase|CallDebussyShoot)
    (CallFunction|DebussyWaitTime)))

(event Custom|DebussyWaitTime
  (Utilities|FlowControl|Delay (Variables|Default|GetWaitTimeDebussy))
  (Variables|Default|SetbDebussyCalled false))

(event EventBeginPlay
  (bind _returnvalue (WorldSubsystems|GetMetaSoundOutputSubsystem))
  (bind _returnvalue_2 (AddComponent|AddAudioComponent false))
  (MetaSoundOutput|WatchOutput _returnvalue _returnvalue_2 "MS_Float_Nyeh_Out" (delegate Custom|Nyeh_Out) "None" "None" :!class /Script/MetasoundEngine.MetaSoundOutputSubsystem)
  (bind _returnvalue_3 (AddComponent|AddAudioComponent false))
  (MetaSoundOutput|WatchOutput _returnvalue _returnvalue_3 "MS_Float_Debussy_Out" (delegate Custom|Debussy_Out) "None" "None" :!class /Script/MetasoundEngine.MetaSoundOutputSubsystem))

(fn ConstructionScript)
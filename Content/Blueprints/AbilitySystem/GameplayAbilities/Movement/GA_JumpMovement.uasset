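; Gameplay Ability for a jump movement that fires when the ability's input is released.
; On release it calls MoveJump, then reads MovementTime from the owner's CubeAttributeSet.
; It waits for MovementTime plus TimeDilation before committing and ending the ability, so the commit happens after the jump has started rather than before it.
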(event Ability|EventActivateAbility
  (Ability|Tasks|WaitInputRelease false
    (:OnRelease
      (Class|MovementGameplayAbility|MoveJump)
      (bind _returnvalue (GameplayAttributes|GetAttributeSet (Ability|GetAbilitySystemComponentfromActorInfo) "/Script/Cube.CubeAttributeSet"))
      (bind _ascube_attribute_set (Utilities|Casting|CastToCubeAttributeSet _returnvalue))
      (bind _output_get (Variables|Default|SetCubeAttributeSet _ascube_attribute_set))
      (Utilities|FlowControl|Delay (+ (.CurrentValue (Utilities|Struct|BreakGameplayAttributeData (Variables|/Script/Cube.CubeAttributeSet|GetMovementTime _output_get))) (Variables|Default|GetTimeDilation)))
      (Ability|CommitAbility)
      (Ability|EndAbility))))

(event Ability|EventOnEndAbility
  (params (bWasCancelled :type Boolean)))
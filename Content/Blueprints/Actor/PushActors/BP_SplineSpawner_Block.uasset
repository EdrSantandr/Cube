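; Spline spawner for blocking push actors that moves its spawned actor along a spline, either once or in a loop.
; Both move events take the spawned actor and drive its world location and rotation from a timeline scaled by spline length, with play rate set by InteractionTime.
; One-shot destroys the actor two seconds after reaching the end; loop ping-pongs by flipping Forward on each finish.
; The spawning logic is not in this graph.
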(event EventBeginPlay
  (|CallParentFunction) ; This node is disabled and will not be called.\nDrag off pins to build functionality.
)

(event Collision|EventActorBeginOverlap
  (params (OtherActor :type Actor%20Object%20Reference))
  (|CallParentFunction OtherActor) ; This node is disabled and will not be called.\nDrag off pins to build functionality.
)

(event EventTick
  (params (DeltaSeconds :type Float%20%28single-precision%29))
  (|CallParentFunction DeltaSeconds) ; This node is disabled and will not be called.\nDrag off pins to build functionality.
)

(event EventMoveSpawnedBlockingOneShot
  ;[1 1 1] OneShotSplineMovable Actor
  (Components|Timeline|SetPlayRate (Variables|Default|GetOneShotTimeline) (/ 1.0 (Variables|Default|GetInteractionTime)))
  (bind _returnvalue (Class|CubeSplineMeshActor|GetSpawnedActor))
  (Variables|Default|SetSplineMovableActor _returnvalue)
  (Variables|Default|SetSplineTotalLength (Spline|GetSplineLength (Variables|Default|GetSplineComponent)))
  (bind _distance (Timeline|OneShotTimeline PlayFromStart)
    (:Update
      (Transformation|SetActorLocationAndRotation (Variables|Default|GetSplineMovableActor) (.Location (Math|Transform|BreakTransform (Spline|GetTransformatDistanceAlongSpline (Variables|Default|GetSplineComponent) (* _distance (Variables|Default|GetSplineTotalLength)) "World" false))) (.Rotation (Math|Transform|BreakTransform (Spline|GetTransformatDistanceAlongSpline (Variables|Default|GetSplineComponent) (* _distance (Variables|Default|GetSplineTotalLength)) "World" false)))))
    (:Finished
      (Development|PrintString "finish")
      (Utilities|FlowControl|Delay 2.0)
      (Actor|DestroyActor (Variables|Default|GetSplineMovableActor)))))

(event EventMoveSpawnedBlockingLoop
  ;[1 1 1] LoopSplineMovable Actor
  (Components|Timeline|SetPlayRate (Variables|Default|GetLoopTimeline) (/ 1.0 (Variables|Default|GetInteractionTime)))
  (bind _returnvalue (Class|CubeSplineMeshActor|GetSpawnedActor))
  (Variables|Default|SetSplineMovableActor _returnvalue)
  (Variables|Default|SetSplineTotalLength (Spline|GetSplineLength (Variables|Default|GetSplineComponent)))
  (if (Variables|Default|GetForward) :!label _label
    (bind _distance (Timeline|LoopTimeline PlayFromStart)
      (:Update
        (Transformation|SetActorLocationAndRotation (Variables|Default|GetSplineMovableActor) (.Location (Math|Transform|BreakTransform (Spline|GetTransformatDistanceAlongSpline (Variables|Default|GetSplineComponent) (* _distance (Variables|Default|GetSplineTotalLength)) "World" false))) (.Rotation (Math|Transform|BreakTransform (Spline|GetTransformatDistanceAlongSpline (Variables|Default|GetSplineComponent) (* _distance (Variables|Default|GetSplineTotalLength)) "World" false)))))
      (:Finished
        (Variables|Default|SetForward (not (Variables|Default|GetForward)))
        (goto _label)))
    (else
      (Timeline|LoopTimeline ReverseFromEnd))))

(fn ConstructionScript
  (|CallParentFunction))
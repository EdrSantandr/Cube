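; BP_PushActor is an actor that shoves the mage player away when they enter its sphere trigger.
; On overlap begin it caches the BP_MagePlayer as a Character and calls PushPlayer; overlap end clears the reference.
; PushPlayer launches the character once along the normalized direction from the actor to the player, scaled by PushForce, adding to existing velocity rather than overriding it.
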(event OnComponentBeginOverlap(Sphere)
  (params (OverlappedComponent :type Primitive%20Component%20Object%20Reference) (OtherActor :type Actor%20Object%20Reference) (OtherComp :type Primitive%20Component%20Object%20Reference) (OtherBodyIndex :type Integer) (bFromSweep :type Boolean) (SweepResult :type Hit%20Result%20Structure%20%28by%20ref%29))
  (Utilities|Casting|CastToBP_MagePlayer OtherActor)
  (bind _ascharacter (Utilities|Casting|CastToCharacter OtherActor))
  (Variables|Default|SetPlayerCharacter _ascharacter)
  (CallFunction|PushPlayer))

(event OnComponentEndOverlap(Sphere)
  (params (OverlappedComponent :type Primitive%20Component%20Object%20Reference) (OtherActor :type Actor%20Object%20Reference) (OtherComp :type Primitive%20Component%20Object%20Reference) (OtherBodyIndex :type Integer))
  (Utilities|Casting|CastToBP_MagePlayer OtherActor)
  (Variables|Default|SetPlayerCharacter 0))

(event EventBeginPlay)

(event Collision|EventActorBeginOverlap
  (params (OtherActor :type Actor%20Object%20Reference)))

(event EventTick
  (params (DeltaSeconds :type Float%20%28single-precision%29)))

(fn ConstructionScript)

(fn PushPlayer
  (bind _output_get (LocalVariables|SetDirection (Math|Vector|Normalize (- (Transformation|GetActorLocation (Variables|Default|GetPlayerCharacter)) (Transformation|GetActorLocation)))))
  (Character|LaunchCharacter (Variables|Default|GetPlayerCharacter) (* _output_get (Variables|Default|GetPushForce)) false false))
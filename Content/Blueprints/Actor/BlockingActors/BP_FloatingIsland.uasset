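; BP_FloatingIsland is a moving island actor that periodically changes direction, driven by a ProjectileMovementComponent.
; On BeginPlay it randomizes initial speed and max speed separately within a shared range, then picks a random bounce interval.
; A looping timer calls ChangeDirection, which multiplies velocity by the negated VelocityDirection to produce the bounce without Tick.
; The timer is cleared when the actor is destroyed.
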(event Custom|ChangeDirection
  (bind _projectilemovementcomponent (Variables|Default|GetProjectileMovementComponent))
  (Variables|/Script/Engine.MovementComponent|SetVelocity _projectilemovementcomponent (* (Variables|/Script/Engine.MovementComponent|GetVelocity _projectilemovementcomponent) (* (Variables|Default|GetVelocityDirection) -1.0))))

(event EventBeginPlay
  (bind _projectilemovementcomponent (Variables|Default|GetProjectileMovementComponent))
  (|CallParentFunction)
  (Variables|/Script/Engine.ProjectileMovementComponent|SetInitialSpeed _projectilemovementcomponent (Math|Random|RandomFloatinRange (Variables|Default|GetMinSpeed) (Variables|Default|GetMaxSpeed)))
  (Variables|/Script/Engine.ProjectileMovementComponent|SetMaxSpeed _projectilemovementcomponent (Math|Random|RandomFloatinRange (Variables|Default|GetMinSpeed) (Variables|Default|GetMaxSpeed)))
  (bind _output_get (Variables|Default|SetBounceTimeDelay (Math|Random|RandomFloatinRange (Variables|Default|GetMinBounceTime) (Variables|Default|GetMaxBounceTime))))
  (bind _returnvalue (Utilities|Time|SetTimerbyEvent (delegate Custom|ChangeDirection) _output_get true))
  (Variables|Default|SetBouncingTimerHandle _returnvalue))

(event Collision|EventActorBeginOverlap
  (params (OtherActor :type Actor%20Object%20Reference))
  (|CallParentFunction OtherActor) ; This node is disabled and will not be called.\nDrag off pins to build functionality.
)

(event EventTick
  (params (DeltaSeconds :type Float%20%28single-precision%29))
  (|CallParentFunction DeltaSeconds) ; This node is disabled and will not be called.\nDrag off pins to build functionality.
)

(event EventDestroyed
  (Utilities|Time|ClearandInvalidateTimerbyHandle (Variables|Default|GetBouncingTimerHandle)))

(fn ConstructionScript
  (|CallParentFunction))